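; Zombie character that walks toward a point ahead of its spawn facing and dies from any damage, regardless of amount.
; BeginPlay computes that destination once and issues a single AI MoveTo.
; AnyDamage stores the damage causer and calls Die, which ragdolls the mesh and launches it along the causer's forward vector.
; Death also disables movement and capsule collision, then destroys the actor after a short delay.
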(event `self.ReceiveBeginPlay`
  (set `self.targetPos` (+ (`self.K2_GetActorLocation`) (* (`KismetMathLibrary.GetForwardVector` (`self.K2_GetActorRotation`)) 1000.0)))
  (`self.MoveTo`))

(event `self.ReceiveAnyDamage`
  (params (Damage :type "Float (single-precision)") (DamageType :type "DamageType Object Reference") (InstigatedBy :type "Controller Object Reference") (DamageCauser :type "Actor Object Reference"))
  (set `self.Damage Causer` DamageCauser)
  (`self.Die`))

(event `Die`
  (bind _mesh (`self.Mesh`))
  (`|ExecutionSequence`
    (:`then_0`
      (`PrimitiveComponent.SetCollisionEnabled` _mesh "QueryAndPhysics")
      (`PrimitiveComponent.SetSimulatePhysics` _mesh true)
      (`SkeletalMeshComponent.SetPhysicsBlendWeight` _mesh 1.0)
      (`PrimitiveComponent.AddImpulse` (`self.Mesh`) (* (`self.GetActorForwardVector` (`self.Damage Causer`)) 3000.0) "None" true))
    (:`then_1`
      (`CharacterMovementComponent.DisableMovement` (`self.CharacterMovement`))
      (`PrimitiveComponent.SetCollisionEnabled` (`self.CapsuleComponent`) "NoCollision"))
    (:`then_2`
      (`KismetSystemLibrary.Delay` 3.0)
      (`self.K2_DestroyActor`))))

(event `MoveTo`
  (`|AIMoveTo` self (`self.targetPos`) null))

(fn `UserConstructionScript`)